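; PaintTarget is a destructible target that awards the player a point when destroyed.
; CollisionSphere overlaps from anything except RuntimeCubeActor reduce its hit points; at zero it increments the FirstPersonCharacter's score and destroys itself.
; SpawnCollision counts overlapping RuntimeCubeActor walls.
; While any overlap, Tick sets its location to the scaled, horizontal player-to-target direction as an absolute position, without adding the current location.
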(event `self.ReceiveBeginPlay`
  (bind _output_get (set `self.hpMax` 3.0))
  (set `self.hitPoints` _output_get))

(event `self.CollisionSphere.OnComponentBeginOverlap`
  (params (OverlappedComponent :type "PrimitiveComponent Object Reference") (OtherActor :type "Actor Object Reference") (OtherComp :type "PrimitiveComponent Object Reference") (OtherBodyIndex :type Integer) (bFromSweep :type Boolean) (SweepResult :type "HitResult Structure (by ref)"))
  (cast `RuntimeCubeActor` OtherActor
    (:`CastFailed`
      (bind _result (`/Engine/EditorBlueprintResources/StandardMacros.DecrementFloat` (`self.hitPoints`))
        (:`  `
          (if (<= _result 0.0)
            (bind _asfirst_person_character (cast `/Game/FirstPersonCPP/Blueprints/FirstPersonCharacter` (`GameplayStatics.GetPlayerCharacter` 0)))
            (set `/Game/FirstPersonCPP/Blueprints/FirstPersonCharacter.Score` (+ (`/Game/FirstPersonCPP/Blueprints/FirstPersonCharacter.Score` _asfirst_person_character) 1) _asfirst_person_character)
            (`self.K2_DestroyActor`)))))))

(event `ExitWallCollision`
  (if (`self.isWallCollision`)
    (bind _asfirst_person_character (cast `/Game/FirstPersonCPP/Blueprints/FirstPersonCharacter` (`GameplayStatics.GetPlayerCharacter` 0)))
    (`self.K2_SetActorLocation` (* (* (`KismetMathLibrary.Normal` (- (`self.K2_GetActorLocation`) (`self.K2_GetActorLocation` _asfirst_person_character))) (1.0 1.0 0.0)) 5.0))))

(event `self.ReceiveTick`
  (params (DeltaSeconds :type "Float (single-precision)"))
  (`self.ExitWallCollision`))

(event `self.SpawnCollision.OnComponentBeginOverlap`
  (params (OverlappedComponent :type "PrimitiveComponent Object Reference") (OtherActor :type "Actor Object Reference") (OtherComp :type "PrimitiveComponent Object Reference") (OtherBodyIndex :type Integer) (bFromSweep :type Boolean) (SweepResult :type "HitResult Structure (by ref)"))
  (cast `RuntimeCubeActor` OtherActor)
  (set `self.isWallCollision` true)
  (`/Engine/EditorBlueprintResources/StandardMacros.IncrementInt` (`self.wallsColliding`)))

(event `self.SpawnCollision.OnComponentEndOverlap`
  (params (OverlappedComponent :type "PrimitiveComponent Object Reference") (OtherActor :type "Actor Object Reference") (OtherComp :type "PrimitiveComponent Object Reference") (OtherBodyIndex :type Integer))
  (bind _wallscolliding (`self.wallsColliding`))
  (cast `RuntimeCubeActor` OtherActor)
  (`/Engine/EditorBlueprintResources/StandardMacros.DecrementInt` _wallscolliding
    (:`  `
      (if (not (> _wallscolliding 0))
        (set `self.isWallCollision` false)))))

(fn `UserConstructionScript`)